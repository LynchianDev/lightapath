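; BP_Interactable_Base is a base Actor for interactable objects that shows a floating text prompt.
; EnteredRange and ExitedRange show and hide the TextRender component, and Interact is left empty.
; While the text is visible, Tick calls FaceCamera, which yaws it toward the player camera using a look-at rotation.
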(event EventBeginPlay)

(event Collision|EventActorBeginOverlap
  (params (OtherActor :type Actor%20Object%20Reference)))

(event EventTick
  (params (DeltaSeconds :type Float%20%28single-precision%29))
  (if (Variables|/Script/Engine.SceneComponent|GetbVisible (Variables|Default|GetTextRender))
    (CallFunction|FaceCamera)))

(event EventEnteredRange
  (Rendering|SetVisibility (Variables|Default|GetTextRender) true false))

(event EventExitedRange
  (Rendering|SetVisibility (Variables|Default|GetTextRender) false false))

(event EventInteract)

(fn ConstructionScript)

(fn FaceCamera
  (bind _textrender (Variables|Default|GetTextRender))
  (Transformation|SetWorldRotation _textrender (Math|Rotator|MakeRotator 0.0 0.0 (.yaw (Math|Rotator|FindLookatRotation (Transformation|GetWorldLocation _textrender) (Camera|GetCameraLocation (Game|GetPlayerCameraManager 0))))) false false))