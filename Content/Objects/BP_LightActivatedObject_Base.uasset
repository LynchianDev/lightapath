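; Base Blueprint for an object with a light-sensitive crystal that activates when it has line of sight to a lamp.
; Entering light stores the lamp and starts a looping timer, apparently driving a Visibility trace from crystal to lamp.
; A Destructible-type hit activates it and rescales the crystal, while other hit types deactivate it.
; Exiting light clears the timer and, only if active, deactivates and resets the lamp and DoOnce.
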(event Custom|CheckLineOfSightToLamp
  (bind _outhit (Collision|LineTraceByChannel (Transformation|GetWorldLocation (Variables|Default|GetLightSensitiveCrystal)) (Transformation|GetWorldLocation (Variables|/Game/Objects/Lamp/BP_Lamp.BP_Lamp_C|GetCube (Variables|Default|GetLamp))) "TraceTypeQuery1" false 0 "None"))
  (Utilities|IsValid (.hitcomponent _outhit)
    (:Is%20Valid
      (if (Utilities|Enum|Equal(Enum) (Collision|GetCollisionObjectType (.hitcomponent _outhit)) "ECC_Destructible")
        (Development|PrintString "Activate")
        (CallFunction|Activate)
        (elif (Variables|Default|GetIsActive)
          (Development|PrintString "Deactivate")
          (CallFunction|Deactivate)
          (else
            (Development|PrintString "not destructible")))))
    (:Is%20Not%20Valid
      (Development|PrintString "lintrace doesnt hit"))))

(event Custom|Activate
  (Variables|Default|SetIsActive true)
  (Transformation|SetRelativeScale3D (Variables|Default|GetLightSensitiveCrystal) "0.700000,0.300000,0.300000"))

(event Custom|Deactivate
  (Variables|Default|SetIsActive false)
  (Transformation|SetRelativeScale3D (Variables|Default|GetLightSensitiveCrystal) "0.100000,0.300000,0.300000"))

(event EventBeginPlay)

(event Collision|EventActorBeginOverlap
  (params (OtherActor :type Actor%20Object%20Reference)))

(event EventTick
  (params (DeltaSeconds :type Float%20%28single-precision%29)))

(event EventEnteredLight
  (params (LampEntered :type BP%20Lamp%20Object%20Reference))
  (Variables|Default|SetLamp LampEntered)
  (Development|PrintString "Hello")
  (Utilities|FlowControl|DoOnce false
    (:Completed
      (bind _returnvalue (Utilities|Time|SetTimerbyEvent (EventDispatchers|CreateEvent :!event Custom|CheckLineOfSightToLamp) 0.1 true))
      (Variables|Default|SetLineOfSightCheck _returnvalue))))

(event EventExitedLight
  (params (LampExited :type BP%20Lamp%20Object%20Reference))
  (Utilities|Time|ClearandInvalidateTimerbyHandle (Variables|Default|GetLineOfSightCheck))
  (if (Variables|Default|GetIsActive)
    (Development|PrintString "Deactivate")
    (CallFunction|Deactivate)
    (Variables|Default|SetLamp 0)
    (Utilities|FlowControl|DoOnce false) ; enters at Reset
  ))

(fn ConstructionScript)