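; Light-activated door that raises on Activate and lowers on Deactivate, moving the Door component over a 200-unit vertical range.
; Each move captures the current door location and uses its own timeline to lerp Z from it.
; Two DoOnce gates interlock the moves: finishing the opening re-arms closing and finishing the closing re-arms opening, so repeated triggers do not restart a move.
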(event EventBeginPlay
  (|CallParentFunction) ; This node is disabled and will not be called.\nDrag off pins to build functionality.
)

(event Collision|EventActorBeginOverlap
  (params (OtherActor :type Actor%20Object%20Reference))
  (|CallParentFunction OtherActor) ; This node is disabled and will not be called.\nDrag off pins to build functionality.
)

(event EventTick
  (params (DeltaSeconds :type Float%20%28single-precision%29))
  (|CallParentFunction DeltaSeconds) ; This node is disabled and will not be called.\nDrag off pins to build functionality.
)

(event EventActivate
  (Utilities|FlowControl|DoOnce false
    (:Completed
      (Variables|Default|SetNewVar_0 (Transformation|GetWorldLocation (Variables|Default|GetDoor)))
      (bind _moveup (Timeline|Timeline_0 PlayFromStart)
        (:Update
          (Transformation|SetWorldLocation (Variables|Default|GetDoor) (Math|Vector|MakeVector (.x (Variables|Default|GetNewVar_0)) (.y (Variables|Default|GetNewVar_0)) (Math|Float|Lerp (.z (Variables|Default|GetNewVar_0)) (+ (.z (Variables|Default|GetNewVar_0)) 2e+02) _moveup)) false false))
        (:Finished
          (Utilities|FlowControl|DoOnce false) ; enters at Reset
        )))))

(event EventDeactivate
  (Utilities|FlowControl|DoOnce false
    (:Completed
      (Variables|Default|SetNewVar_0 (Transformation|GetWorldLocation (Variables|Default|GetDoor)))
      (bind _moveup (Timeline|Timeline_1 PlayFromStart)
        (:Update
          (Transformation|SetWorldLocation (Variables|Default|GetDoor) (Math|Vector|MakeVector (.x (Variables|Default|GetNewVar_0)) (.y (Variables|Default|GetNewVar_0)) (Math|Float|Lerp (+ (.z (Variables|Default|GetNewVar_0)) -2e+02) (.z (Variables|Default|GetNewVar_0)) _moveup)) false false))
        (:Finished
          (Utilities|FlowControl|DoOnce false) ; enters at Reset
        )))))

(fn ConstructionScript
  (|CallParentFunction))