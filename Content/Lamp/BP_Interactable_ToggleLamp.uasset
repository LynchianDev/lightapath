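; Interactable lamp actor that toggles a child BP_Lamp and draws the player camera toward it.
; Interact and a duplicate Togglerino event both call Toggle on the lamp and set IsControlled, which this graph never clears.
; While IsControlled is set, Tick moves the player camera manager itself toward the lamp's CamPos with VInterpTo, rather than switching view target.
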(event Custom|Togglerino
  (bind _asbp_lamp (Utilities|Casting|CastToBP_Lamp (Variables|/Script/Engine.ChildActorComponent|GetChildActor (Variables|Default|GetLamp))))
  (Default|Toggle _asbp_lamp)
  (Variables|Default|SetIsControlled true))

(event EventBeginPlay
  (|CallParentFunction) ; This node is disabled and will not be called.\nDrag off pins to build functionality.
)

(event Collision|EventActorBeginOverlap
  (params (OtherActor :type Actor%20Object%20Reference))
  (|CallParentFunction OtherActor) ; This node is disabled and will not be called.\nDrag off pins to build functionality.
)

(event EventTick
  (params (DeltaSeconds :type Float%20%28single-precision%29))
  (bind _returnvalue (Game|GetPlayerCameraManager 0))
  (|CallParentFunction DeltaSeconds)
  (if (Variables|Default|GetIsControlled)
    (bind _asbp_lamp (Utilities|Casting|CastToBP_Lamp (Variables|/Script/Engine.ChildActorComponent|GetChildActor (Variables|Default|GetLamp))))
    (Transformation|SetActorLocation _returnvalue (Math|Interpolation|VInterpTo (Camera|GetCameraLocation _returnvalue) (Transformation|GetWorldLocation (Variables|/Game/Lamp/BP_Lamp.BP_Lamp_C|GetCamPos _asbp_lamp)) (Utilities|Time|GetWorldDeltaSeconds) 1e+01) false false)))

(event EventInteract
  (bind _asbp_lamp (Utilities|Casting|CastToBP_Lamp (Variables|/Script/Engine.ChildActorComponent|GetChildActor (Variables|Default|GetLamp))))
  (Default|Toggle _asbp_lamp)
  (Variables|Default|SetIsControlled true))

(fn ConstructionScript
  (|CallParentFunction))