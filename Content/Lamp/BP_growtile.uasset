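; BP_growtile is a tile that grows and shrinks, apparently as a reaction to lamp light.
; Activate stretches its Cube component vertically into a tall pillar, and Deactivate returns it to a small cube, both as instant scale changes.
; EnteredLight and ExitedLight only forward to the parent class, so any link between light and activation lies outside this Blueprint.
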(event EventBeginPlay
  (|CallParentFunction) ; This node is disabled and will not be called.\nDrag off pins to build functionality.
)

(event Collision|EventActorBeginOverlap
  (params (OtherActor :type Actor%20Object%20Reference))
  (|CallParentFunction OtherActor) ; This node is disabled and will not be called.\nDrag off pins to build functionality.
)

(event EventTick
  (params (DeltaSeconds :type Float%20%28single-precision%29))
  (|CallParentFunction DeltaSeconds) ; This node is disabled and will not be called.\nDrag off pins to build functionality.
)

(event EventExitedLight
  (params (LampExited :type BP%20Lamp%20Object%20Reference))
  (|CallParentFunction LampExited))

(event EventEnteredLight
  (params (LampEntered :type BP%20Lamp%20Object%20Reference))
  (|CallParentFunction LampEntered))

(event EventDeactivate
  (Transformation|SetRelativeScale3D (Variables|Default|GetCube) "0.300000,0.300000,0.300000"))

(event EventActivate
  (Transformation|SetRelativeScale3D (Variables|Default|GetCube) "0.300000,0.300000,1.800000"))

(fn ConstructionScript
  (|CallParentFunction))