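; Actor with a light-sensitive crystal that switches on when it has line of sight to a lamp whose light it entered.
; Entering light stores the lamp and starts a looping timer, apparently for visibility traces from crystal to lamp.
; A hit on a Destructible-type component activates it, stretching its cube, while other hits shrink it.
; Exiting light stops the timer, deactivates and clears the lamp.
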(event Custom|CheckLineOfSightToLamp
  (bind _outhit (Collision|LineTraceByChannel (Transformation|GetWorldLocation (Variables|Default|GetLightSensitiveCrystal)) (Transformation|GetWorldLocation (Variables|/Game/Lamp/BP_Lamp.BP_Lamp_C|GetCube (Variables|Default|GetLamp))) "TraceTypeQuery1" false 0 "None"))
  (Utilities|IsValid (.hitcomponent _outhit)
    (:Is%20Valid
      (Development|PrintString (Utilities|GetObjectName (.hitactor _outhit)))
      (if (Utilities|Enum|Equal(Enum) (Collision|GetCollisionObjectType (.hitcomponent _outhit)) "ECC_Destructible")
        (CallFunction|Activate)
        (else
          (CallFunction|Deactivate))))
    (:Is%20Not%20Valid
      (Development|PrintString "lintrace doesnt hit"))))

(event Custom|Activate
  (Transformation|SetRelativeScale3D (Variables|Default|GetCube) "2.000000,0.300000,0.300000"))

(event Custom|Deactivate
  (Transformation|SetRelativeScale3D (Variables|Default|GetCube) "0.100000,0.300000,0.300000"))

(event EventBeginPlay)

(event Collision|EventActorBeginOverlap
  (params (OtherActor :type Actor%20Object%20Reference)))

(event EventTick
  (params (DeltaSeconds :type Float%20%28single-precision%29)))

(event EventEnteredLight
  (params (LampEntered :type BP%20Lamp%20Object%20Reference))
  (Variables|Default|SetLamp LampEntered)
  (Utilities|FlowControl|DoOnce false
    (:Completed
      (bind _returnvalue (Utilities|Time|SetTimerbyEvent (EventDispatchers|CreateEvent :!event Custom|CheckLineOfSightToLamp) 0.1 true))
      (Variables|Default|SetLineOfSightCheck _returnvalue))))

(event EventExitedLight
  (params (LampExited :type BP%20Lamp%20Object%20Reference))
  (Utilities|Time|ClearandInvalidateTimerbyHandle (Variables|Default|GetLineOfSightCheck))
  (CallFunction|Deactivate)
  (Variables|Default|SetLamp 0)
  (Utilities|FlowControl|DoOnce false) ; enters at Reset
)

(fn ConstructionScript)